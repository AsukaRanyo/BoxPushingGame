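; BP_Destination is a flow actor that marks where BP_Box actors stop.
; When any actor begins overlapping its Box component, it prints that actor's class name.
; If the actor is a BP_Box, it sets IsStop on it and calls SetState, leaving the resulting behavior to the box.
; BeginPlay, Tick and the construction script are empty.
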(event `self.Box.OnComponentBeginOverlap`
  (params (OverlappedComponent :type "PrimitiveComponent Object Reference") (OtherActor :type "Actor Object Reference") (OtherComp :type "PrimitiveComponent Object Reference") (OtherBodyIndex :type Integer) (bFromSweep :type Boolean) (SweepResult :type "HitResult Structure (by ref)"))
  (set `self.Other Actor` OtherActor)
  (`KismetSystemLibrary.PrintString` (`KismetSystemLibrary.GetClassDisplayName` (`GameplayStatics.GetObjectClass` OtherActor)))
  (if (`GameplayStatics.ObjectIsA` (`self.Other Actor`) "/Game/BluePrint/Flow/BP_Box.BP_Box_C")
    (bind _asbp_box (cast `/Game/BluePrint/Flow/BP_Box` (`self.Other Actor`)))
    (set `/Game/BluePrint/Flow/BP_Box.IsStop` true _asbp_box)
    (`/Game/BluePrint/Flow/BP_Box.SetState` _asbp_box)))

(fn `UserConstructionScript`)