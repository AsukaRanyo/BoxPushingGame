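; Pushable Sokoban-style box that the third-person character shoves one grid cell at a time, completing the level when no goals remain.
; Four side overlap triggers set the push direction, debounced by a short timer.
; The target cell is checked in GameInstance level data: walls and boxes block, otherwise the data updates and the box moves.
; Covered goals become Clear; once all are, the next numbered level opens.
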(event `SetState`
  (if (`self.IsStop`)
    (`SceneComponent.SetVisibility` (`self.Niagara1`) false false)))

(event `self.BoxFront.OnComponentBeginOverlap`
  (params (OverlappedComponent :type "PrimitiveComponent Object Reference") (OtherActor :type "Actor Object Reference") (OtherComp :type "PrimitiveComponent Object Reference") (OtherBodyIndex :type Integer) (bFromSweep :type Boolean) (SweepResult :type "HitResult Structure (by ref)"))
  (if (and (`GameplayStatics.ObjectIsA` OtherActor "/Game/ThirdPerson/Blueprints/BP_ThirdPersonCharacter.BP_ThirdPersonCharacter_C") (not (`self.IsStop`)))
    (bind _output_get (set `self.CollisionDirection` "NewEnumerator1"))
    (`self.CollisionHanding` _output_get)
    (`KismetSystemLibrary.PrintString` "发生碰撞")
    (`GameplayStatics.PlaySound2D` "/Game/StarterContent/Audio/Explosion01.Explosion01" 1.0 1.0 0.0 null null)))

(event `self.BoxBack.OnComponentBeginOverlap`
  (params (OverlappedComponent :type "PrimitiveComponent Object Reference") (OtherActor :type "Actor Object Reference") (OtherComp :type "PrimitiveComponent Object Reference") (OtherBodyIndex :type Integer) (bFromSweep :type Boolean) (SweepResult :type "HitResult Structure (by ref)"))
  (if (and (`GameplayStatics.ObjectIsA` OtherActor "/Game/ThirdPerson/Blueprints/BP_ThirdPersonCharacter.BP_ThirdPersonCharacter_C") (not (`self.IsStop`)))
    (bind _output_get (set `self.CollisionDirection` "NewEnumerator2"))
    (`self.CollisionHanding` _output_get)
    (`KismetSystemLibrary.PrintString` "发生碰撞")
    (`GameplayStatics.PlaySound2D` "/Game/StarterContent/Audio/Explosion01.Explosion01" 1.0 1.0 0.0 null null)))

(event `self.BoxRight.OnComponentBeginOverlap`
  (params (OverlappedComponent :type "PrimitiveComponent Object Reference") (OtherActor :type "Actor Object Reference") (OtherComp :type "PrimitiveComponent Object Reference") (OtherBodyIndex :type Integer) (bFromSweep :type Boolean) (SweepResult :type "HitResult Structure (by ref)"))
  (if (and (`GameplayStatics.ObjectIsA` OtherActor "/Game/ThirdPerson/Blueprints/BP_ThirdPersonCharacter.BP_ThirdPersonCharacter_C") (not (`self.IsStop`)))
    (bind _output_get (set `self.CollisionDirection` "NewEnumerator3"))
    (`self.CollisionHanding` _output_get)
    (`KismetSystemLibrary.PrintString` "发生碰撞")
    (`GameplayStatics.PlaySound2D` "/Game/StarterContent/Audio/Explosion01.Explosion01" 1.0 1.0 0.0 null null)))

(event `self.BoxLeft.OnComponentBeginOverlap`
  (params (OverlappedComponent :type "PrimitiveComponent Object Reference") (OtherActor :type "Actor Object Reference") (OtherComp :type "PrimitiveComponent Object Reference") (OtherBodyIndex :type Integer) (bFromSweep :type Boolean) (SweepResult :type "HitResult Structure (by ref)"))
  (if (and (`GameplayStatics.ObjectIsA` OtherActor "/Game/ThirdPerson/Blueprints/BP_ThirdPersonCharacter.BP_ThirdPersonCharacter_C") (not (`self.IsStop`)))
    (bind _output_get (set `self.CollisionDirection` "NewEnumerator4"))
    (`self.CollisionHanding` _output_get)
    (`KismetSystemLibrary.PrintString` "发生碰撞")
    (`GameplayStatics.PlaySound2D` "/Game/StarterContent/Audio/Explosion01.Explosion01" 1.0 1.0 0.0 null null)))

(fn `ArrayFind`
  (params (X :type Integer) (Y :type Integer))
  (returns (ArrayIndex :type Integer) (NewParam :type "/Game/BluePrint/Structure/S_GameStructure Structure"))
  (`KismetSystemLibrary.PrintString` (`KismetStringLibrary.Concat_StrStr` "x=" (`KismetStringLibrary.Conv_IntToString` X) "组x=" (`KismetStringLibrary.Conv_IntToString` (`.X_10_3A87BD1644F0C022572D4D8C61277E2C` (break `/Game/BluePrint/Structure/S_GameStructure` (stale _array_element)))) "，" "" (`KismetStringLibrary.Conv_IntToString` Y) "" (`KismetStringLibrary.Conv_IntToString` (`.Y_9_FCF219BE4EBEB9A6C156FDABCDAD17FB` (break `/Game/BluePrint/Structure/S_GameStructure` (stale _array_element))))))
  (for (_array_element _array_index) (`self.LevelData`)
    (if (and (== (`.X_10_3A87BD1644F0C022572D4D8C61277E2C` (break `/Game/BluePrint/Structure/S_GameStructure` _array_element)) X) (== (`.Y_9_FCF219BE4EBEB9A6C156FDABCDAD17FB` (break `/Game/BluePrint/Structure/S_GameStructure` _array_element)) Y))
      (`KismetSystemLibrary.PrintString` "找到数据" true true (struct :`R` 1.0 :`G` 0.005154 :`B` 0.015101 :`A` 1.0))
      (set `self.SGame` (make `/Game/BluePrint/Structure/S_GameStructure` (break `/Game/BluePrint/Structure/S_GameStructure` _array_element) (`.X_10_3A87BD1644F0C022572D4D8C61277E2C` (break `/Game/BluePrint/Structure/S_GameStructure` _array_element)) (`.Y_9_FCF219BE4EBEB9A6C156FDABCDAD17FB` (break `/Game/BluePrint/Structure/S_GameStructure` _array_element)) (`.ActorType_11_A0149D6445ADC8176611A9A67D10D6FC` (break `/Game/BluePrint/Structure/S_GameStructure` _array_element))))
      (break)))
  (return _array_index (`self.SGame`)))

(fn `CheckFinishLevel`
  (set `self.LevelNum` 2)
  (set `self.IsFinishLevel` true)
  (for _array_element (`self.LevelData`)
    (switch `/Game/BluePrint/Enum/E_ActorType` (`.ActorType_11_A0149D6445ADC8176611A9A67D10D6FC` (break `/Game/BluePrint/Structure/S_GameStructure` _array_element))
      (:`NewEnumerator4`
        (set `self.IsFinishLevel` false)
        (break))))
  (if (`self.IsFinishLevel`)
    (`KismetSystemLibrary.PrintString` "Finishing!")
    (`GameplayStatics.PlaySound2D` "/Game/StarterContent/Audio/Collapse01.Collapse01" 1.0 1.0 0.0 null null)
    (bind _returnvalue (`GameplayStatics.GetCurrentLevelName` true))
    (bind _output_get (set `self.Right S` (`.RightS` (`KismetStringLibrary.Split` _returnvalue "evel"))))
    (bind _result (`/Engine/EditorBlueprintResources/StandardMacros.IncrementInt` (`KismetStringLibrary.Conv_StringToInt` _output_get))
      (:`  `
        (if true
          (`GameplayStatics.OpenLevel` (`KismetStringLibrary.Conv_StringToName` (`KismetStringLibrary.Concat_StrStr` "Level" (`KismetStringLibrary.Conv_IntToString` _result))))
          (else
            (`GameplayStatics.OpenLevel` "Level0")))))))

(fn `CheckNextPoint`
  (returns (IsMove :type Boolean))
  (bind _checkcollisiondirection (`self.CheckCollisionDirection`))
  (`KismetSystemLibrary.PrintString` (`|GetEnumeratorNameAsString` _checkcollisiondirection))
  (switch `/Game/BluePrint/Enum/ECollisionDirection` _checkcollisiondirection
    (:`NewEnumerator1`
      (bind _newparam (`self.CheckNextPointType` (- (`self.LocationX`) 1) (`self.LocationY`)))
      (return _newparam))
    (:`NewEnumerator2`
      (bind _newparam_2 (`self.CheckNextPointType` (+ (`self.LocationX`) 1) (`self.LocationY`)))
      (return _newparam_2))
    (:`NewEnumerator3`
      (bind _newparam_3 (`self.CheckNextPointType` (`self.LocationX`) (- (`self.LocationY`) 1)))
      (return _newparam_3))
    (:`NewEnumerator4`
      (bind _newparam_4 (`self.CheckNextPointType` (`self.LocationX`) (+ (`self.LocationY`) 1)))
      (return _newparam_4))))

(fn `CheckNextPointType`
  (params (X :type Integer) (Y :type Integer))
  (returns (NewParam :type Boolean))
  (bind _array_index (`self.Array Index`))
  (set `self.X` X)
  (set `self.Y` Y)
  (`|ExecutionSequence`
    (:`then_0`
      (`KismetSystemLibrary.PrintString` (`KismetStringLibrary.Concat_StrStr` "X=" (`KismetStringLibrary.Conv_IntToString` (`self.X`)) "," "Y=" (`KismetStringLibrary.Conv_IntToString` (`self.Y`)) "Then 0"))
      (bind _asbp_game_instrance (cast `/Game/BluePrint/GameInstrance/BP_GameInstrance` (`GameplayStatics.GetGameInstance`)))
      (bind _leveldata (`/Game/BluePrint/GameInstrance/BP_GameInstrance.GetLevelDataGI` _asbp_game_instrance))
      (set `self.LevelData` _leveldata))
    (:`then_1`
      (bind (_arrayindex _newparam) (`self.ArrayFind` (`self.X`) (`self.Y`)))
      (set `self.Array Index` _arrayindex)
      (`KismetSystemLibrary.PrintString` (`|GetEnumeratorNameAsString` (`.ActorType_11_A0149D6445ADC8176611A9A67D10D6FC` (break `/Game/BluePrint/Structure/S_GameStructure` _newparam))))
      (switch `/Game/BluePrint/Enum/E_ActorType` (`.ActorType_11_A0149D6445ADC8176611A9A67D10D6FC` (break `/Game/BluePrint/Structure/S_GameStructure` _newparam))
        (:`NewEnumerator2`
          _)
        (:`NewEnumerator3`
          _)
        (:`NewEnumerator4`
          (`KismetArrayLibrary.Array_Set` (`self.LevelData`) _array_index (make `/Game/BluePrint/Structure/S_GameStructure` 1 (`self.X`) (`self.Y`) "NewEnumerator1"))
          (`KismetSystemLibrary.PrintString` (`KismetStringLibrary.Concat_StrStr` "X=" (`KismetStringLibrary.Conv_IntToString` (`self.X`)) "," "Y=" (`KismetStringLibrary.Conv_IntToString` (`self.Y`)) "Index：" (`KismetStringLibrary.Conv_IntToString` _array_index)))
          (`GameplayStatics.PlaySound2D` "/Game/StarterContent/Audio/Collapse01.Collapse01" 1.0 1.0 0.0 null null)
          (bind _arrayindex_2 (`self.ArrayFind` (`self.LocationX`) (`self.LocationY`) :!label _label))
          (`KismetArrayLibrary.Array_Set` (`self.LevelData`) _arrayindex_2 (make `/Game/BluePrint/Structure/S_GameStructure` 0 (`self.LocationX`) (`self.LocationY`) "NewEnumerator6"))
          (set `self.LocationX` (`self.X`))
          (set `self.LocationY` (`self.Y`))
          (bind _asbp_game_instrance_2 (cast `/Game/BluePrint/GameInstrance/BP_GameInstrance` (`GameplayStatics.GetGameInstance`)))
          (`/Game/BluePrint/GameInstrance/BP_GameInstrance.SetLevelDataGI` _asbp_game_instrance_2 (`self.LevelData`))
          (return true))
        (:`NewEnumerator5`
          (`KismetArrayLibrary.Array_Set` (`self.LevelData`) (`self.Array Index`) (make `/Game/BluePrint/Structure/S_GameStructure` 1 (`self.X`) (`self.Y`) "NewEnumerator3") :!label _label_2)
          (goto _label))
        (:`NewEnumerator6`
          (`KismetSystemLibrary.PrintString` "can")
          (goto _label_2)))
      (return false))))

(fn `CollisionHanding`
  (params (CollisionDirection :type "/Game/BluePrint/Enum/ECollisionDirection Enum" :default "NewEnumerator0"))
  (bind (_returnvalue_x _returnvalue_y _returnvalue_z) (`KismetMathLibrary.BreakVector` (`self.K2_GetActorLocation` self)))
  (bind (_returnvalue_x_2 _returnvalue_y_2 _returnvalue_z_2) (`KismetMathLibrary.BreakVector` (`self.K2_GetActorLocation` self)))
  (bind (_returnvalue_x_3 _returnvalue_y_3 _returnvalue_z_3) (`KismetMathLibrary.BreakVector` (`self.K2_GetActorLocation` self)))
  (bind (_returnvalue_x_4 _returnvalue_y_4 _returnvalue_z_4) (`KismetMathLibrary.BreakVector` (`self.K2_GetActorLocation` self)))
  (set `self.CheckCollisionDirection` CollisionDirection)
  (if (not (`self.IsCollisionIng`))
    (set `self.IsCollisionIng` true)
    (`KismetSystemLibrary.K2_SetTimer` null "SelfSCollision" 0.1)
    (switch `/Game/BluePrint/Enum/ECollisionDirection` CollisionDirection
      (:`NewEnumerator1`
        (`KismetSystemLibrary.PrintString` "前碰撞" true true (struct :`G` 0.66 :`B` 1.0 :`A` 1.0) 5.0)
        (bind _ismove (`self.CheckNextPoint`))
        (if _ismove
          (`KismetSystemLibrary.PrintString` "Hello")
          (`self.K2_SetActorLocation` self (`KismetMathLibrary.MakeVector` (- _returnvalue_x_4 100.0) _returnvalue_y_4 _returnvalue_z_4) false false)
          (set `self.CollisionDirection` "NewEnumerator0")
          (`self.CheckFinishLevel` :!label _label)))
      (:`NewEnumerator2`
        (`KismetSystemLibrary.PrintString` "后碰撞" true true (struct :`G` 0.66 :`B` 1.0 :`A` 1.0) 5.0)
        (bind _ismove_2 (`self.CheckNextPoint`))
        (if _ismove_2
          (`self.K2_SetActorLocation` self (`KismetMathLibrary.MakeVector` (+ _returnvalue_x_2 100.0) _returnvalue_y_2 _returnvalue_z_2) false false)
          (set `self.CollisionDirection` "NewEnumerator0")
          (goto _label)))
      (:`NewEnumerator3`
        (`KismetSystemLibrary.PrintString` "右碰撞" true true (struct :`G` 0.66 :`B` 1.0 :`A` 1.0) 5.0)
        (bind _ismove_3 (`self.CheckNextPoint`))
        (if _ismove_3
          (`self.K2_SetActorLocation` self (`KismetMathLibrary.MakeVector` _returnvalue_x_3 (- _returnvalue_y_3 100.0) _returnvalue_z_3) false false)
          (set `self.CollisionDirection` "NewEnumerator0")
          (goto _label)))
      (:`NewEnumerator4`
        (`KismetSystemLibrary.PrintString` "左碰撞" true true (struct :`G` 0.66 :`B` 1.0 :`A` 1.0) 5.0)
        (bind _ismove_4 (`self.CheckNextPoint`))
        (if _ismove_4
          (`self.K2_SetActorLocation` self (`KismetMathLibrary.MakeVector` _returnvalue_x (+ _returnvalue_y 100.0) _returnvalue_z) false false)
          (set `self.CollisionDirection` "NewEnumerator0")
          (goto _label))))))

(fn `SelfSCollision`
  (set `self.IsCollisionIng` false))

(fn `UserConstructionScript`
  (`SceneComponent.SetVisibility` (`self.Niagara1`) true false)
  (set `self.IsStop` false)
  (set `self.IsCollisionIng` false))